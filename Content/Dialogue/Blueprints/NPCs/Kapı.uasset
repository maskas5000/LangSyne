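; Door ("Kapı") set up as a dialogue NPC, tied to the Gamemode's BuffDudeDoorOpened flag.
; Interact stores the instigator and opens the DialogueKapı conversation, then closes it after a minimal delay if that flag is set.
; BeginPlay starts a looping timer on an empty Opened event, and the flag check and capsule-destroy nodes left in the graph are disconnected.
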(event Custom|Opened)

(event EventInteract
  (params (Instigator :type Actor%20Object%20Reference))
  (Variables|Default|SetInteractInstigator Instigator)
  (Default|OpenConversation (Variables|Default|GetDialogue_Kapı))
  (if (Variables|/Game/TopDown/Blueprints/BP_TopDownGameMode.BP_TopDownGameMode_C|GetBuffDudeDoorOpened (Variables|/Game/Dialogue/Blueprints/Dialogues/AC_Dialogue_Base.AC_Dialogue_Base_C|GetGamemode (Variables|Default|GetDialogue_Kapı)))
    (Utilities|FlowControl|Delay 0.001)
    (Default|CloseConversation (Variables|Default|GetDialogue_Kapı))))

(event EventBeginPlay
  (Utilities|Time|SetTimerbyFunctionName 0 "Opened" 0.2 true))

(fn ConstructionScript
  (|CallParentFunction))