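; Dialogue Blueprint for the first echo scene at the bar, where Lyen, troubled by a headache and a garbled Echoed Voice, resolves to investigate Little Joe, a lead from a dream.
; It extends a parent dialogue class, calling the parent's gamemode lookup on BeginPlay and the parent Dialogue before its own lines.
; The script is a linear chain of AddDialogue nodes, each with a single Continue option, ending in CloseConversation.
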(event EventBeginPlay
  (CallFunction|GetGamemode))

(fn GetGamemode
  (|CallParentFunction))

(fn Dialogue
  (|CallParentFunction)
  (bind (_state _optionindex) (CallFunction|AddDialogue "Lyen" "Ugh, its that headache again..." (Utilities|Array|MakeArray "Continue")))
  (switch Utilities|FlowControl|Switch|SwitchonEnum_DialogueState _state
    (:NewEnumerator0
      (switch int _optionindex
        (:0
          (bind (_state_2 _optionindex_2) (CallFunction|AddDialogue "Echoed Voice" "Br......n m.....t ke... ....e..r ....om..." (Utilities|Array|MakeArray "Continue")))
          (switch Utilities|FlowControl|Switch|SwitchonEnum_DialogueState _state_2
            (:NewEnumerator0
              (switch int _optionindex_2
                (:0
                  (bind (_state_3 _optionindex_3) (CallFunction|AddDialogue "Lyen" "Huh?!" (Utilities|Array|MakeArray "Continue")))
                  (switch Utilities|FlowControl|Switch|SwitchonEnum_DialogueState _state_3
                    (:NewEnumerator0
                      (switch int _optionindex_3
                        (:0
                          (bind (_state_4 _optionindex_4) (CallFunction|AddDialogue "Lyen" "Where is that voice coming from?" (Utilities|Array|MakeArray "Continue")))
                          (switch Utilities|FlowControl|Switch|SwitchonEnum_DialogueState _state_4
                            (:NewEnumerator0
                              (switch int _optionindex_4
                                (:0
                                  (bind (_state_5 _optionindex_5) (CallFunction|AddDialogue "Lyen" "Whatever, I came here for a reason. I need to figure out who this Little Joe person is." (Utilities|Array|MakeArray "Continue")))
                                  (switch Utilities|FlowControl|Switch|SwitchonEnum_DialogueState _state_5
                                    (:NewEnumerator0
                                      (switch int _optionindex_5
                                        (:0
                                          (bind (_state_6 _optionindex_6) (CallFunction|AddDialogue "Lyen" "Can’t believe I am chasing a lead that I saw in my dream." (Utilities|Array|MakeArray "Continue")))
                                          (switch Utilities|FlowControl|Switch|SwitchonEnum_DialogueState _state_6
                                            (:NewEnumerator0
                                              (switch int _optionindex_6
                                                (:0
                                                  (bind (_state_7 _optionindex_7) (CallFunction|AddDialogue "Lyen" "But everything has been accurate thus far." (Utilities|Array|MakeArray "Continue")))
                                                  (switch Utilities|FlowControl|Switch|SwitchonEnum_DialogueState _state_7
                                                    (:NewEnumerator0
                                                      (switch int _optionindex_7
                                                        (:0
                                                          (bind (_state_8 _optionindex_8) (CallFunction|AddDialogue "Lyen" "But everything has been accurate thus far." (Utilities|Array|MakeArray "Continue")))
                                                          (switch Utilities|FlowControl|Switch|SwitchonEnum_DialogueState _state_8
                                                            (:NewEnumerator0
                                                              (switch int _optionindex_8
                                                                (:0
                                                                  (bind (_state_9 _optionindex_9) (CallFunction|AddDialogue "Lyen" "Okay I have made up my mind. I will go in there and investigate the lead." (Utilities|Array|MakeArray "Continue")))
                                                                  (switch Utilities|FlowControl|Switch|SwitchonEnum_DialogueState _state_9
                                                                    (:NewEnumerator0
                                                                      (switch int _optionindex_9
                                                                        (:0
                                                                          (bind (_state_10 _optionindex_10) (CallFunction|AddDialogue "Lyen" "Better start asking around." (Utilities|Array|MakeArray "Continue")))
                                                                          (switch Utilities|FlowControl|Switch|SwitchonEnum_DialogueState _state_10
                                                                            (:NewEnumerator0
                                                                              (switch int _optionindex_10
                                                                                (:0
                                                                                  (bind (_state_11 _optionindex_11) (CallFunction|AddDialogue "Echoed Voice " "Yes..." (Utilities|Array|MakeArray "Continue")))
                                                                                  (switch Utilities|FlowControl|Switch|SwitchonEnum_DialogueState _state_11
                                                                                    (:NewEnumerator0
                                                                                      (switch int _optionindex_11
                                                                                        (:0
                                                                                          (bind (_state_12 _optionindex_12) (CallFunction|AddDialogue "Lyen" "Huh?.." (Utilities|Array|MakeArray "Continue")))
                                                                                          (switch Utilities|FlowControl|Switch|SwitchonEnum_DialogueState _state_12
                                                                                            (:NewEnumerator0
                                                                                              (switch int _optionindex_12
                                                                                                (:0
                                                                                                  (CallFunction|CloseConversation))))))))))))))))))))))))))))))))))))))))))))))))))