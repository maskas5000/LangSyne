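; Dialogue Blueprint for a bar patron and her friends, branching on the Gamemode's TimeSlot.
; In the first slot, asking about Elisha (offered with KeyA) earns an invitation, setting KeyB and a local flag that shortens repeat talks.
; In the second, KeyB admits Lyen to the group, where Key2 unlocks an Iron Hounds question that sets KeyC; without KeyB she is rebuffed.
; Lines are chained AddDialogue calls, with shared branches looping back to the topic menu.
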(event EventBeginPlay
  (CallFunction|GetGamemode))

(event EventTick
  (params (DeltaSeconds :type Float%20%28single-precision%29)))

(fn Dialogue
  (|CallParentFunction)
  (switch int (Variables|/Game/TopDown/Blueprints/BP_TopDownGameMode.BP_TopDownGameMode_C|GetTimeSlot (Variables|Default|GetGamemode))
    (:0
      (if (Variables|Default|GetTS1ConvoHappened)
        (bind (_state _optionindex) (CallFunction|AddDialogue "Lyen" "İ got what i need." (Utilities|Array|MakeArray "Continue")))
        (switch Utilities|FlowControl|Switch|SwitchonEnum_DialogueState _state
          (:NewEnumerator0
            (switch int _optionindex
              (:0
                (CallFunction|ClearDialogueProgress)
                (CallFunction|CloseConversation)))))
        (else
          (bind (_state_2 _optionindex_2) (CallFunction|AddDialogue "Woman 1" "Uhhhh is there something on my face, why are you staring like a creep." (Utilities|Array|MakeArray "No, I just wanted to talk." "Sorry I didn’t mean to (Leave)")))
          (switch Utilities|FlowControl|Switch|SwitchonEnum_DialogueState _state_2
            (:NewEnumerator0
              (switch int _optionindex_2
                (:0
                  (bind (_state_3 _optionindex_3) (CallFunction|AddDialogue "Woman 1" "Uhhh like, what do you wanna talk about." (Utilities|Array|MakeArray "Any gossip around here lately?")))
                  (switch Utilities|FlowControl|Switch|SwitchonEnum_DialogueState _state_3
                    (:NewEnumerator0
                      (switch int _optionindex_3
                        (:0
                          (bind (_state_4 _optionindex_4) (CallFunction|AddDialogue "Woman 1" "I meaaaan, I don’t really know much." (Utilities|Array|MakeArray "Continue")))
                          (switch Utilities|FlowControl|Switch|SwitchonEnum_DialogueState _state_4
                            (:NewEnumerator0
                              (switch int _optionindex_4
                                (:0
                                  (if (Variables|/Game/TopDown/Blueprints/BP_TopDownGameMode.BP_TopDownGameMode_C|GetKeyA (Variables|Default|GetGamemode)) :!label _label
                                    (bind (_state_5 _optionindex_5) (CallFunction|AddDialogue "Woman 1" "I only come here because I know the bartender’s wife and he gives me free stuff sometimes." (Utilities|Array|MakeArray "Oh you know Elisha too? How is she? " "So you never heard anything about Little Joe?" "Do you know anything else about this place?" "I have to leave now. (Leave)")))
                                    (switch Utilities|FlowControl|Switch|SwitchonEnum_DialogueState _state_5
                                      (:NewEnumerator0
                                        (switch int _optionindex_5
                                          (:0
                                            (bind (_state_6 _optionindex_6) (CallFunction|AddDialogue "Woman 1" "Dear she is doing amazing from what I have heard." (Utilities|Array|MakeArray "Continue")))
                                            (switch Utilities|FlowControl|Switch|SwitchonEnum_DialogueState _state_6
                                              (:NewEnumerator0
                                                (switch int _optionindex_6
                                                  (:0
                                                    (bind (_state_7 _optionindex_7) (CallFunction|AddDialogue "Woman 1" "I haven’t seen her in a while though, I should go visit sometime." (Utilities|Array|MakeArray "Continue")))
                                                    (switch Utilities|FlowControl|Switch|SwitchonEnum_DialogueState _state_7
                                                      (:NewEnumerator0
                                                        (switch int _optionindex_7
                                                          (:0
                                                            (bind (_state_8 _optionindex_8) (CallFunction|AddDialogue "Woman 1" "Yknow what, I have some friends coming over in a hot minute. You should come visit us then. I would love to introduce you to them." (Utilities|Array|MakeArray "Continue")))
                                                            (switch Utilities|FlowControl|Switch|SwitchonEnum_DialogueState _state_8
                                                              (:NewEnumerator0
                                                                (switch int _optionindex_8
                                                                  (:0
                                                                    (Variables|/Game/TopDown/Blueprints/BP_TopDownGameMode.BP_TopDownGameMode_C|SetKeyB (Variables|Default|GetGamemode) true)
                                                                    (Variables|Default|SetTS1ConvoHappened true)
                                                                    (CallFunction|ClearDialogueProgress)
                                                                    (CallFunction|CloseConversation))))))))))))))
                                          (:1
                                            (bind (_state_9 _optionindex_9) (CallFunction|AddDialogue "Woman 1" "I know the name, but so does anyone who lives around here." (Utilities|Array|MakeArray "Continue") :!label _label_2))
                                            (switch Utilities|FlowControl|Switch|SwitchonEnum_DialogueState _state_9
                                              (:NewEnumerator0
                                                (switch int _optionindex_9
                                                  (:0
                                                    (bind (_state_10 _optionindex_10) (CallFunction|AddDialogue "Woman 1" "Wish I could help but all I know is that he likes to hang around in this bar sometimes." (Utilities|Array|MakeArray "Continue")))
                                                    (switch Utilities|FlowControl|Switch|SwitchonEnum_DialogueState _state_10
                                                      (:NewEnumerator0
                                                        (switch int _optionindex_10
                                                          (:0
                                                            (goto _label))))))))))
                                          (:2
                                            (bind (_state_11 _optionindex_11) (CallFunction|AddDialogue "Woman 1" "They opened a new diner just across this place. I heard their food it to die for." (Utilities|Array|MakeArray "Thanks, might as well go check it out sometime.") :!label _label_3))
                                            (switch Utilities|FlowControl|Switch|SwitchonEnum_DialogueState _state_11
                                              (:NewEnumerator0
                                                (switch int _optionindex_11
                                                  (:0
                                                    (goto _label))))))
                                          (:3
                                            (CallFunction|ClearDialogueProgress :!label _label_4)
                                            (CallFunction|CloseConversation)))))
                                    (else
                                      (bind (_state_12 _optionindex_12) (CallFunction|AddDialogue "Woman 1" "I only come here because I know the bartender’s wife and he gives me free stuff sometimes." (Utilities|Array|MakeArray "So you never heard anything about Little Joe?" "Do you know anything else about this place?" "I have to leave now. (Leave)")))
                                      (switch Utilities|FlowControl|Switch|SwitchonEnum_DialogueState _state_12
                                        (:NewEnumerator0
                                          (switch int _optionindex_12
                                            (:0
                                              (goto _label_2))
                                            (:1
                                              (goto _label_3))
                                            (:2
                                              (goto _label_4))))))))))))))))
                (:1
                  (CallFunction|ClearDialogueProgress)
                  (CallFunction|CloseConversation))))))))
    (:1
      (if (Variables|/Game/TopDown/Blueprints/BP_TopDownGameMode.BP_TopDownGameMode_C|GetKeyB (Variables|Default|GetGamemode))
        (bind (_state_13 _optionindex_13) (CallFunction|AddDialogue "Woman 1" "Uhhhh is there something on my face, why are you staring like a creep." (Utilities|Array|MakeArray "Would you look at that, you actually came.")))
        (switch Utilities|FlowControl|Switch|SwitchonEnum_DialogueState _state_13
          (:NewEnumerator0
            (switch int _optionindex_13
              (:0
                (bind (_state_14 _optionindex_14) (CallFunction|AddDialogue "Woman 1" "Everyone, this is... Uh..." (Utilities|Array|MakeArray "Lyen, I am a friend of Elisha’s.")))
                (switch Utilities|FlowControl|Switch|SwitchonEnum_DialogueState _state_14
                  (:NewEnumerator0
                    (switch int _optionindex_14
                      (:0
                        (bind (_state_15 _optionindex_15) (CallFunction|AddDialogue "Woman 1" "Yes, thats right." (Utilities|Array|MakeArray "Continue")))
                        (switch Utilities|FlowControl|Switch|SwitchonEnum_DialogueState _state_15
                          (:NewEnumerator0
                            (switch int _optionindex_15
                              (:0
                                (bind (_state_16 _optionindex_16) (CallFunction|AddDialogue "Woman 2" "Please come sit, I have never seen you around here. Did you just move to this part of the city?" (Utilities|Array|MakeArray "Yeah, sure.")))
                                (switch Utilities|FlowControl|Switch|SwitchonEnum_DialogueState _state_16
                                  (:NewEnumerator0
                                    (switch int _optionindex_16
                                      (:0
                                        (bind (_state_17 _optionindex_17) (CallFunction|AddDialogue "Woman 3" "Where did you live before?" (Utilities|Array|MakeArray "In Torenn Alley, just cross the Red Falcon Precinct.")))
                                        (switch Utilities|FlowControl|Switch|SwitchonEnum_DialogueState _state_17
                                          (:NewEnumerator0
                                            (switch int _optionindex_17
                                              (:0
                                                (bind (_state_18 _optionindex_18) (CallFunction|AddDialogue "Woman 2" "It must have been such an upgrade moving to here." (Utilities|Array|MakeArray "Continue.")))
                                                (switch Utilities|FlowControl|Switch|SwitchonEnum_DialogueState _state_18
                                                  (:NewEnumerator0
                                                    (switch int _optionindex_18
                                                      (:0
                                                        (bind (_state_19 _optionindex_19) (CallFunction|AddDialogue "Woman 2" "Even the air tastes different in this part of the city." (Utilities|Array|MakeArray "Continue.")))
                                                        (switch Utilities|FlowControl|Switch|SwitchonEnum_DialogueState _state_19
                                                          (:NewEnumerator0
                                                            (switch int _optionindex_19
                                                              (:0
                                                                (bind (_state_20 _optionindex_20) (CallFunction|AddDialogue "Woman 3" "I mean... There is the occasional shoot-out, but you get used to that." (Utilities|Array|MakeArray "Continue.")))
                                                                (switch Utilities|FlowControl|Switch|SwitchonEnum_DialogueState _state_20
                                                                  (:NewEnumerator0
                                                                    (switch int _optionindex_20
                                                                      (:0
                                                                        (bind (_state_21 _optionindex_21) (CallFunction|AddDialogue "Woman 2" "Mhm, when I first came here I thought I was gonna end up dead on the street. But the thing is gangs only want to fight with each other." (Utilities|Array|MakeArray "Continue.")))
                                                                        (switch Utilities|FlowControl|Switch|SwitchonEnum_DialogueState _state_21
                                                                          (:NewEnumerator0
                                                                            (switch int _optionindex_21
                                                                              (:0
                                                                                (if (Variables|/Game/TopDown/Blueprints/BP_TopDownGameMode.BP_TopDownGameMode_C|GetKey2 (Variables|Default|GetGamemode))
                                                                                  (bind (_state_22 _optionindex_22) (CallFunction|AddDialogue "Woman 2" "They don’t really want aynthing from you so you can relax, yknow." (Utilities|Array|MakeArray "Thanks, thats all very helpful. (Leave)" "But I heard things have been getting worse, with the Iron Hounds trying to expand their territory and all.")))
                                                                                  (switch Utilities|FlowControl|Switch|SwitchonEnum_DialogueState _state_22
                                                                                    (:NewEnumerator0
                                                                                      (switch int _optionindex_22
                                                                                        (:0
                                                                                          (CallFunction|ClearDialogueProgress :!label _label_5)
                                                                                          (CallFunction|CloseConversation))
                                                                                        (:1
                                                                                          (bind (_state_23 _optionindex_23) (CallFunction|AddDialogue "Woman 1" "Yeah I heard that as well. My prayers go to Elisha." (Utilities|Array|MakeArray "Continue")))
                                                                                          (switch Utilities|FlowControl|Switch|SwitchonEnum_DialogueState _state_23
                                                                                            (:NewEnumerator0
                                                                                              (switch int _optionindex_23
                                                                                                (:0
                                                                                                  (bind (_state_24 _optionindex_24) (CallFunction|AddDialogue "Woman 2" "It’s already hard to carry a baby, but now she might give birth anytime and there is a whole gang war on the streets. " (Utilities|Array|MakeArray "Continue")))
                                                                                                  (switch Utilities|FlowControl|Switch|SwitchonEnum_DialogueState _state_24
                                                                                                    (:NewEnumerator0
                                                                                                      (switch int _optionindex_24
                                                                                                        (:0
                                                                                                          (bind (_state_25 _optionindex_25) (CallFunction|AddDialogue "Woman 3" "Must be tough..." (Utilities|Array|MakeArray "Continue")))
                                                                                                          (switch Utilities|FlowControl|Switch|SwitchonEnum_DialogueState _state_25
                                                                                                            (:NewEnumerator0
                                                                                                              (switch int _optionindex_25
                                                                                                                (:0
                                                                                                                  (Variables|/Game/TopDown/Blueprints/BP_TopDownGameMode.BP_TopDownGameMode_C|SetKeyC (Variables|Default|GetGamemode) true)
                                                                                                                  (CallFunction|ClearDialogueProgress)
                                                                                                                  (CallFunction|CloseConversation)))))))))))))))))
                                                                                  (else
                                                                                    (bind (_state_26 _optionindex_26) (CallFunction|AddDialogue "Woman 2" "They don’t really want aynthing from you so you can relax, yknow." (Utilities|Array|MakeArray "Thanks, thats all very helpful. (Leave)")))
                                                                                    (switch Utilities|FlowControl|Switch|SwitchonEnum_DialogueState _state_26
                                                                                      (:NewEnumerator0
                                                                                        (switch int _optionindex_26
                                                                                          (:0
                                                                                            (goto _label_5)))))))))))))))))))))))))))))))))))))))))))
        (else
          (bind (_state_27 _optionindex_27) (CallFunction|AddDialogue "Woman 2" "Who is this this? Did any of you invite her?" (Utilities|Array|MakeArray "Continue")))
          (switch Utilities|FlowControl|Switch|SwitchonEnum_DialogueState _state_27
            (:NewEnumerator0
              (switch int _optionindex_27
                (:0
                  (bind (_state_28 _optionindex_28) (CallFunction|AddDialogue "Woman 3" "No clue love, maybe we should ask her." (Utilities|Array|MakeArray "Continue")))
                  (switch Utilities|FlowControl|Switch|SwitchonEnum_DialogueState _state_28
                    (:NewEnumerator0
                      (switch int _optionindex_28
                        (:0
                          (bind (_state_29 _optionindex_29) (CallFunction|AddDialogue "Woman 1" "Noo, she is just some random girl." (Utilities|Array|MakeArray "Continue")))
                          (switch Utilities|FlowControl|Switch|SwitchonEnum_DialogueState _state_29
                            (:NewEnumerator0
                              (switch int _optionindex_29
                                (:0
                                  (bind (_state_30 _optionindex_30) (CallFunction|AddDialogue "Woman 1" "Hey, stop bothering me and my friends" (Utilities|Array|MakeArray "Leave")))
                                  (switch Utilities|FlowControl|Switch|SwitchonEnum_DialogueState _state_30
                                    (:NewEnumerator0
                                      (switch int _optionindex_30
                                        (:0
                                          (CallFunction|ClearDialogueProgress)
                                          (CallFunction|CloseConversation))))))))))))))))))))))

(fn GetGamemode
  (|CallParentFunction))