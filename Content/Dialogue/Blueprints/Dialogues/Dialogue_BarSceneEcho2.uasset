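; Scripted conversation for the second bar-scene echo, where Lyen meets the "Good" echo, a cloud of fragments bound to the shattered watch.
; The voice introduces the rival "Bad" and "Ugly" echoes and an unknown promise to keep.
; The Dialogue override calls its parent, then chains single-option AddDialogue steps linearly until CloseConversation, with one "use us" line appearing twice in succession.
; BeginPlay only runs GetGamemode, which defers to the parent.
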(event EventBeginPlay
  (CallFunction|GetGamemode))

(fn Dialogue
  (|CallParentFunction)
  (bind (_state _optionindex) (CallFunction|AddDialogue "Lyen" "Ouch, my head hurts like hell." (Utilities|Array|MakeArray "Continue")))
  (switch Utilities|FlowControl|Switch|SwitchonEnum_DialogueState _state
    (:NewEnumerator0
      (switch int _optionindex
        (:0
          (bind (_state_2 _optionindex_2) (CallFunction|AddDialogue "Echoed Voice" "B..ken one, we ...ust speak." (Utilities|Array|MakeArray "That voice... It is getting closer and closer.")))
          (switch Utilities|FlowControl|Switch|SwitchonEnum_DialogueState _state_2
            (:NewEnumerator0
              (switch int _optionindex_2
                (:0
                  (bind (_state_3 _optionindex_3) (CallFunction|AddDialogue "Echoed Voice" "Broken one, we must speak. We must keep their promise." (Utilities|Array|MakeArray "W-Who are you?")))
                  (switch Utilities|FlowControl|Switch|SwitchonEnum_DialogueState _state_3
                    (:NewEnumerator0
                      (switch int _optionindex_3
                        (:0
                          (bind (_state_4 _optionindex_4) (CallFunction|AddDialogue "Echoed Voice" "I am one of many. And I speak for most." (Utilities|Array|MakeArray "Yeah, because that makes a lot more sense.")))
                          (switch Utilities|FlowControl|Switch|SwitchonEnum_DialogueState _state_4
                            (:NewEnumerator0
                              (switch int _optionindex_4
                                (:0
                                  (bind (_state_5 _optionindex_5) (CallFunction|AddDialogue "Echoed Voice" "It’s alright we will explain." (Utilities|Array|MakeArray "Continue")))
                                  (switch Utilities|FlowControl|Switch|SwitchonEnum_DialogueState _state_5
                                    (:NewEnumerator0
                                      (switch int _optionindex_5
                                        (:0
                                          (bind (_state_6 _optionindex_6) (CallFunction|AddDialogue "Echoed Voice" "We are fragments of the people who once held this watch." (Utilities|Array|MakeArray "Continue")))
                                          (switch Utilities|FlowControl|Switch|SwitchonEnum_DialogueState _state_6
                                            (:NewEnumerator0
                                              (switch int _optionindex_6
                                                (:0
                                                  (bind (_state_7 _optionindex_7) (CallFunction|AddDialogue "Echoed Voice" "When it was shattered we broke free. But we cannot get away from the watch." (Utilities|Array|MakeArray "Continue")))
                                                  (switch Utilities|FlowControl|Switch|SwitchonEnum_DialogueState _state_7
                                                    (:NewEnumerator0
                                                      (switch int _optionindex_7
                                                        (:0
                                                          (bind (_state_8 _optionindex_8) (CallFunction|AddDialogue "Echoed Voice" "Something was promised to us. We want it." (Utilities|Array|MakeArray "What was the promised thing.")))
                                                          (switch Utilities|FlowControl|Switch|SwitchonEnum_DialogueState _state_8
                                                            (:NewEnumerator0
                                                              (switch int _optionindex_8
                                                                (:0
                                                                  (bind (_state_9 _optionindex_9) (CallFunction|AddDialogue "Echoed Voice" "We don’t know yet. We think that you will find it for us." (Utilities|Array|MakeArray "So what did you mean when you said “I speak for the most”. Are there those who don’t agree with you.")))
                                                                  (switch Utilities|FlowControl|Switch|SwitchonEnum_DialogueState _state_9
                                                                    (:NewEnumerator0
                                                                      (switch int _optionindex_9
                                                                        (:0
                                                                          (bind (_state_10 _optionindex_10) (CallFunction|AddDialogue "Echoed Voice" "When we told you that we were fragments. I really meant it." (Utilities|Array|MakeArray "Continue")))
                                                                          (switch Utilities|FlowControl|Switch|SwitchonEnum_DialogueState _state_10
                                                                            (:NewEnumerator0
                                                                              (switch int _optionindex_10
                                                                                (:0
                                                                                  (bind (_state_11 _optionindex_11) (CallFunction|AddDialogue "Echoed Voice" "We have been here so long that we lost where we come from. Most fragments just find a “characteristic” to reside under." (Utilities|Array|MakeArray "Continue")))
                                                                                  (switch Utilities|FlowControl|Switch|SwitchonEnum_DialogueState _state_11
                                                                                    (:NewEnumerator0
                                                                                      (switch int _optionindex_11
                                                                                        (:0
                                                                                          (bind (_state_12 _optionindex_12) (CallFunction|AddDialogue "Echoed Voice" "You can refer to the cloud of fragments that you are talking to as “Good”." (Utilities|Array|MakeArray "Continue")))
                                                                                          (switch Utilities|FlowControl|Switch|SwitchonEnum_DialogueState _state_12
                                                                                            (:NewEnumerator0
                                                                                              (switch int _optionindex_12
                                                                                                (:0
                                                                                                  (bind (_state_13 _optionindex_13) (CallFunction|AddDialogue "Echoed Voice" "We are one of the three major echos inside. The other two are the “Bad” and the “Ugly”." (Utilities|Array|MakeArray "Continue")))
                                                                                                  (switch Utilities|FlowControl|Switch|SwitchonEnum_DialogueState _state_13
                                                                                                    (:NewEnumerator0
                                                                                                      (switch int _optionindex_13
                                                                                                        (:0
                                                                                                          (bind (_state_14 _optionindex_14) (CallFunction|AddDialogue "Echoed Voice" "There are many other minor voices but they don’t support you, yet. They think the person that broke the watch can never keep the promise." (Utilities|Array|MakeArray "I am not even the person who broke the watch. I was shot, it saved me.")))
                                                                                                          (switch Utilities|FlowControl|Switch|SwitchonEnum_DialogueState _state_14
                                                                                                            (:NewEnumerator0
                                                                                                              (switch int _optionindex_14
                                                                                                                (:0
                                                                                                                  (bind (_state_15 _optionindex_15) (CallFunction|AddDialogue "Echoed Voice - Good " "We know. But they don’t. You will show them." (Utilities|Array|MakeArray "So what am i supposed to do exactly.")))
                                                                                                                  (switch Utilities|FlowControl|Switch|SwitchonEnum_DialogueState _state_15
                                                                                                                    (:NewEnumerator0
                                                                                                                      (switch int _optionindex_15
                                                                                                                        (:0
                                                                                                                          (bind (_state_16 _optionindex_16) (CallFunction|AddDialogue "Echoed Voice - Good" "For now, use us. Everytime you come here, choose one of the major echos. Slowly you will convince the rest. They will join your seach." (Utilities|Array|MakeArray "Do you think my search has something to do with your promise?")))
                                                                                                                          (switch Utilities|FlowControl|Switch|SwitchonEnum_DialogueState _state_16
                                                                                                                            (:NewEnumerator0
                                                                                                                              (switch int _optionindex_16
                                                                                                                                (:0
                                                                                                                                  (bind (_state_17 _optionindex_17) (CallFunction|AddDialogue "Echoed Voice - Good " "For now, use us. Everytime you come here, choose one of the major echos. Slowly you will convince the rest. They will join your seach." (Utilities|Array|MakeArray "Do you think my search has something to do with your promise?")))
                                                                                                                                  (switch Utilities|FlowControl|Switch|SwitchonEnum_DialogueState _state_17
                                                                                                                                    (:NewEnumerator0
                                                                                                                                      (switch int _optionindex_17
                                                                                                                                        (:0
                                                                                                                                          (bind (_state_18 _optionindex_18) (CallFunction|AddDialogue "Echoed Voice - Good" "In some sense, we could argue that everything is connected. Some things more than others. This is one of those things." (Utilities|Array|MakeArray "Alright but you have to tell me what this watch is.")))
                                                                                                                                          (switch Utilities|FlowControl|Switch|SwitchonEnum_DialogueState _state_18
                                                                                                                                            (:NewEnumerator0
                                                                                                                                              (switch int _optionindex_18
                                                                                                                                                (:0
                                                                                                                                                  (bind (_state_19 _optionindex_19) (CallFunction|AddDialogue "Echoed Voice - Good" "Not now, soon." (Utilities|Array|MakeArray "Continue")))
                                                                                                                                                  (switch Utilities|FlowControl|Switch|SwitchonEnum_DialogueState _state_19
                                                                                                                                                    (:NewEnumerator0
                                                                                                                                                      (switch int _optionindex_19
                                                                                                                                                        (:0
                                                                                                                                                          (CallFunction|CloseConversation))))))))))))))))))))))))))))))))))))))))))))))))))))))))))))))))))))))))))))))

(fn GetGamemode
  (|CallParentFunction))