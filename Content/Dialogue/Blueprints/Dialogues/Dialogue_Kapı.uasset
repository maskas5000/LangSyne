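; Dialogue Blueprint for the door (Kapı) guarded by Buff Dude, who decides whether the player may enter.
; GetGamemode runs on BeginPlay, and Dialogue branches on the game mode's Key1 flag while BuffDudeDoorOpened is false.
; With Key1, the player cites Gil, is let in, and BuffDudeDoorOpened is set; without it, Lyen is turned away.
; Both exchanges end by clearing dialogue progress and closing the conversation.
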(event EventBeginPlay
  (CallFunction|GetGamemode))

(fn Dialogue
  (bind _gamemode (Variables|Default|GetGamemode))
  (|CallParentFunction)
  (if (not (Variables|/Game/TopDown/Blueprints/BP_TopDownGameMode.BP_TopDownGameMode_C|GetBuffDudeDoorOpened _gamemode))
    (if (Variables|/Game/TopDown/Blueprints/BP_TopDownGameMode.BP_TopDownGameMode_C|GetKey1 _gamemode)
      (bind (_state _optionindex) (CallFunction|AddDialogue "Buff Dude" "Who are you?" (Utilities|Array|MakeArray "Gil sent me. Said I should look for the boss.")))
      (switch Utilities|FlowControl|Switch|SwitchonEnum_DialogueState _state
        (:NewEnumerator0
          (switch int _optionindex
            (:0
              (bind _state_2 (CallFunction|AddDialogue "Buff Dude" "In, wait by the table. He will come." (Utilities|Array|MakeArray "Continue")))
              (switch Utilities|FlowControl|Switch|SwitchonEnum_DialogueState _state_2
                (:NewEnumerator0
                  (Variables|/Game/TopDown/Blueprints/BP_TopDownGameMode.BP_TopDownGameMode_C|SetBuffDudeDoorOpened (Variables|Default|GetGamemode) true)
                  (CallFunction|ClearDialogueProgress)
                  (CallFunction|CloseConversation)))))))
      (else
        (bind (_state_3 _optionindex_2) (CallFunction|AddDialogue "Buff Dude" "Who are you?" (Utilities|Array|MakeArray "I'm Lyen.")))
        (switch Utilities|FlowControl|Switch|SwitchonEnum_DialogueState _state_3
          (:NewEnumerator0
            (switch int _optionindex_2
              (:0
                (bind _state_4 (CallFunction|AddDialogue "Buff Dude" "I don't know you. Go away." (Utilities|Array|MakeArray "Continue")))
                (switch Utilities|FlowControl|Switch|SwitchonEnum_DialogueState _state_4
                  (:NewEnumerator0
                    (CallFunction|ClearDialogueProgress)
                    (CallFunction|CloseConversation)))))))))))

(fn GetGamemode
  (|CallParentFunction))