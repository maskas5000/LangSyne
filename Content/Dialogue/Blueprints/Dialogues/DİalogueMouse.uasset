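; Mouse NPC dialogue Blueprint in which the mouse begs the player for cheese and reacts to whether the player is good or bad.
; It overrides a parent Dialogue function, branching on the game mode's TimeSlot and Good flag, plus DialogueTreeIndex and CheeseGiven.
; Chained AddDialogue nodes advance on Pass Through and branch by chosen option.
; Outcomes can set CheeseGiven or advance TimeSlot, and endings clear progress and close the conversation.
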(event EventBeginPlay
  (CallFunction|GetGamemode))

(fn Dialogue
  (|CallParentFunction)
  (switch int (Variables|/Game/TopDown/Blueprints/BP_TopDownGameMode.BP_TopDownGameMode_C|GetTimeSlot (Variables|Default|GetGamemode))
    (:0
      (if (Variables|/Game/TopDown/Blueprints/BP_TopDownGameMode.BP_TopDownGameMode_C|GetGood (Variables|Default|GetGamemode))
        (switch int (Variables|Default|GetDialogueTreeIndex)
          (:0
            (bind (_state _optionindex) (CallFunction|AddDialogue "Mouse" "Hi, do you have any cheese?" (Utilities|Array|MakeArray "Yes" "No") :!label _label))
            (switch Utilities|FlowControl|Switch|SwitchonEnum_DialogueState _state
              (:NewEnumerator0
                (switch int _optionindex
                  (:0
                    (bind (_state_2 _optionindex_2) (CallFunction|AddDialogue "Mouse" "Ahh, that's great news, can I have some?" (Utilities|Array|MakeArray "Give Cheese" "Keep Cheese" "Why Do you want cheese?")))
                    (switch Utilities|FlowControl|Switch|SwitchonEnum_DialogueState _state_2
                      (:NewEnumerator0
                        (switch int _optionindex_2
                          (:0
                            (bind _state_3 (CallFunction|AddDialogue "Mouse" "Thank you, thank you!! You are so kind!!" (Utilities|Array|MakeArray "Continue")))
                            (switch Utilities|FlowControl|Switch|SwitchonEnum_DialogueState _state_3
                              (:NewEnumerator0
                                (Variables|Default|SetCheeseGiven true)
                                (if (== (Variables|/Game/TopDown/Blueprints/BP_TopDownGameMode.BP_TopDownGameMode_C|GetTimeSlot (Variables|Default|GetGamemode)) 0)
                                  (Variables|/Game/TopDown/Blueprints/BP_TopDownGameMode.BP_TopDownGameMode_C|SetTimeSlot (Variables|Default|GetGamemode) 1))
                                (CallFunction|ClearDialogueProgress)
                                (CallFunction|CloseConversation))))
                          (:1
                            (bind _state_4 (CallFunction|AddDialogue "Mouse" "You big meany!" (Utilities|Array|MakeArray "Continue")))
                            (switch Utilities|FlowControl|Switch|SwitchonEnum_DialogueState _state_4
                              (:NewEnumerator0
                                (CallFunction|ClearDialogueProgress)
                                (CallFunction|CloseConversation))))
                          (:2
                            (bind _state_5 (CallFunction|AddDialogue "Mouse" "Because, I love them!" (Utilities|Array|MakeArray "Continue")))
                            (switch Utilities|FlowControl|Switch|SwitchonEnum_DialogueState _state_5
                              (:NewEnumerator0
                                (goto _label))))))))
                  (:1
                    (bind _state_6 (CallFunction|AddDialogue "Mouse" "Awww, that's a shame, I really want some cheese." (Utilities|Array|MakeArray "Continue") :!label _label_2))
                    (switch Utilities|FlowControl|Switch|SwitchonEnum_DialogueState _state_6
                      (:NewEnumerator0
                        (CallFunction|ClearDialogueProgress)
                        (CallFunction|CloseConversation))))))))
          (:1
            (bind _state_7 (CallFunction|AddDialogue "Mouse" (Utilities|Select :Index (Math|Random|RandomIntegerinRange 0 1) :Option%200 "You are such a nice person!" :Option%201 "Nomm Nomm") (Utilities|Array|MakeArray "Continue")))
            (switch Utilities|FlowControl|Switch|SwitchonEnum_DialogueState _state_7
              (:NewEnumerator0
                (CallFunction|ClearDialogueProgress)
                (CallFunction|CloseConversation)))))
        (else
          (bind (_state_8 _optionindex_3) (CallFunction|AddDialogue "Mouse!" "You seem, bad!" (Utilities|Array|MakeArray "Yes, i'm very bad!" "No i'm not bad!")))
          (switch Utilities|FlowControl|Switch|SwitchonEnum_DialogueState _state_8
            (:NewEnumerator0
              (switch int _optionindex_3
                (:0
                  (bind _state_9 (CallFunction|AddDialogue "Mouse!" "Then, get out!" (Utilities|Array|MakeArray "Continue, (come back in a few hours, he will forget you)")))
                  (switch Utilities|FlowControl|Switch|SwitchonEnum_DialogueState _state_9
                    (:NewEnumerator0
                      (Variables|/Game/TopDown/Blueprints/BP_TopDownGameMode.BP_TopDownGameMode_C|SetTimeSlot (Variables|Default|GetGamemode) 1)
                      (CallFunction|ClearDialogueProgress)
                      (CallFunction|CloseConversation))))
                (:1
                  (bind _state_10 (CallFunction|AddDialogue "Mouse!" "I don't know, i'm not trust you." (Utilities|Array|MakeArray "Continue")))
                  (switch Utilities|FlowControl|Switch|SwitchonEnum_DialogueState _state_10
                    (:NewEnumerator0
                      (CallFunction|ClearDialogueProgress)
                      (CallFunction|CloseConversation))))))))))
    (:1
      (if (Variables|/Game/TopDown/Blueprints/BP_TopDownGameMode.BP_TopDownGameMode_C|GetGood (Variables|Default|GetGamemode))
        (if (Variables|Default|GetCheeseGiven)
          (bind _state_11 (CallFunction|AddDialogue "ME" "I gaved the cheese, i dont need to talk" (Utilities|Array|MakeArray "Continue") :!label _label_3))
          (switch Utilities|FlowControl|Switch|SwitchonEnum_DialogueState _state_11
            (:NewEnumerator0
              (CallFunction|ClearDialogueProgress)
              (CallFunction|CloseConversation)))
          (else
            (bind (_state_12 _optionindex_4) (CallFunction|AddDialogue "Mouse" "You look familiar, anyway do you have cheese?" (Utilities|Array|MakeArray "Give cheese" "no")))
            (switch Utilities|FlowControl|Switch|SwitchonEnum_DialogueState _state_12
              (:NewEnumerator0
                (switch int _optionindex_4
                  (:0
                    (bind _state_13 (CallFunction|AddDialogue "Mouse" "Thanks!!!" (Utilities|Array|MakeArray "Continue")))
                    (switch Utilities|FlowControl|Switch|SwitchonEnum_DialogueState _state_13
                      (:NewEnumerator0
                        (Variables|Default|SetCheeseGiven true)
                        (CallFunction|ClearDialogueProgress)
                        (CallFunction|CloseConversation))))
                  (:1
                    (goto _label_2)))))))
        (elif (Variables|Default|GetCheeseGiven)
          (goto _label_3)
          (else
            (bind _state_14 (CallFunction|AddDialogue "Mouse" "You smell bad. Dont want to talk!" (Utilities|Array|MakeArray "Continue")))
            (switch Utilities|FlowControl|Switch|SwitchonEnum_DialogueState _state_14
              (:NewEnumerator0
                (CallFunction|ClearDialogueProgress)
                (CallFunction|CloseConversation)))))))))

(fn GetGamemode
  (|CallParentFunction))