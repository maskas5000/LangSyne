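; Opening dialogue Blueprint, derived from a parent dialogue class, that asks the main character whether they are good or bad.
; BeginPlay fetches the game mode, and Dialogue calls the parent logic, then adds a line with two options.
; On pass-through, the chosen option sets the game mode's Good flag, then dialogue progress is cleared and the conversation closes.
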(event EventBeginPlay
  (CallFunction|GetGamemode))

(fn Dialogue
  (bind _gamemode (Variables|Default|GetGamemode))
  (|CallParentFunction)
  (bind (_state _optionindex) (CallFunction|AddDialogue "Main Character" "Are you a good or bad?" (Utilities|Array|MakeArray "Good." "Bad.")))
  (switch Utilities|FlowControl|Switch|SwitchonEnum_DialogueState _state
    (:NewEnumerator0
      (switch int _optionindex
        (:0
          (Variables|/Game/TopDown/Blueprints/BP_TopDownGameMode.BP_TopDownGameMode_C|SetGood _gamemode true))
        (:1
          (Variables|/Game/TopDown/Blueprints/BP_TopDownGameMode.BP_TopDownGameMode_C|SetGood _gamemode false)))
      (CallFunction|ClearDialogueProgress)
      (CallFunction|CloseConversation))))

(fn GetGamemode
  (|CallParentFunction))