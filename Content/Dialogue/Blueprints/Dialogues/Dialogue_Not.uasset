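; Conversation Blueprint in which the player reads notes, learns a password and questions Little Joe about a missing detective.
; Dialogue only gives the scene in time slot 2 if PlayerKicked is unset; otherwise no one answers.
; Chained AddDialogue calls set Gamemode.Key2 after the notes, then branch on warning Joe or pleading.
; Both endings set PlayerKicked and close the conversation, but only the warning branch resets TimeSlot to 0.
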(event EventBeginPlay
  (CallFunction|GetGamemode))

(fn GetGamemode
  (|CallParentFunction))

(fn Dialogue
  (|CallParentFunction)
  (switch int (Variables|/Game/TopDown/Blueprints/BP_TopDownGameMode.BP_TopDownGameMode_C|GetTimeSlot (Variables|Default|GetGamemode))
    (:0
      (bind (_state _optionindex) (CallFunction|AddDialogue "Lyen" "No one answers." (Utilities|Array|MakeArray "Continue") :!label _label))
      (switch Utilities|FlowControl|Switch|SwitchonEnum_DialogueState _state
        (:NewEnumerator0
          (switch int _optionindex
            (:0
              (CallFunction|ClearDialogueProgress)
              (CallFunction|CloseConversation))))))
    (:1
      (goto _label))
    (:2
      (if (Variables|/Game/TopDown/Blueprints/BP_TopDownGameMode.BP_TopDownGameMode_C|GetPlayerKicked (Variables|Default|GetGamemode))
        (goto _label)
        (else
          (bind (_state_2 _optionindex_2) (CallFunction|AddDialogue "Narrator" "You look through the notes. The thing that catches your eye most is a letter." (Utilities|Array|MakeArray "Continue")))
          (switch Utilities|FlowControl|Switch|SwitchonEnum_DialogueState _state_2
            (:NewEnumerator0
              (switch int _optionindex_2
                (:0
                  (bind (_state_3 _optionindex_3) (CallFunction|AddDialogue "Narrator" "Appearantly people don’t feel safe. They are worried about Iron Hounds." (Utilities|Array|MakeArray "Continue")))
                  (switch Utilities|FlowControl|Switch|SwitchonEnum_DialogueState _state_3
                    (:NewEnumerator0
                      (switch int _optionindex_3
                        (:0
                          (bind (_state_4 _optionindex_4) (CallFunction|AddDialogue "Narrator" "There is also a note mentioning a spy. If what the note says is true, they sent this spy somewhere. Not too long ago. There is a password. It reads “Sent by: Zael Devin. Need: 3 Favors.”" (Utilities|Array|MakeArray "Continue")))
                          (switch Utilities|FlowControl|Switch|SwitchonEnum_DialogueState _state_4
                            (:NewEnumerator0
                              (switch int _optionindex_4
                                (:0
                                  (Variables|/Game/TopDown/Blueprints/BP_TopDownGameMode.BP_TopDownGameMode_C|SetKey2 (Variables|Default|GetGamemode) true)
                                  (bind (_state_5 _optionindex_5) (CallFunction|AddDialogue "Little Joe" "*muffled*Ah you said Gil sent someone. Hm they didn’t say, huh okay I will see myself." (Utilities|Array|MakeArray "Continue")))
                                  (switch Utilities|FlowControl|Switch|SwitchonEnum_DialogueState _state_5
                                    (:NewEnumerator0
                                      (switch int _optionindex_5
                                        (:0
                                          (bind (_state_6 _optionindex_6) (CallFunction|AddDialogue "Little Joe" "Hello friend. Anything I can do for you?" (Utilities|Array|MakeArray "A friend of mine went missing not too long ago. I need some kind of lead and you might have what I need.")))
                                          (switch Utilities|FlowControl|Switch|SwitchonEnum_DialogueState _state_6
                                            (:NewEnumerator0
                                              (switch int _optionindex_6
                                                (:0
                                                  (bind (_state_7 _optionindex_7) (CallFunction|AddDialogue "Little Joe" "I need more, I can’t work with that." (Utilities|Array|MakeArray "He was a detective. He dissapeared three days ago, this Tuesday. ")))
                                                  (switch Utilities|FlowControl|Switch|SwitchonEnum_DialogueState _state_7
                                                    (:NewEnumerator0
                                                      (switch int _optionindex_7
                                                        (:0
                                                          (bind (_state_8 _optionindex_8) (CallFunction|AddDialogue "Little Joe" "Ohhh no, I am not getting myself involved with does lunatics. Not again." (Utilities|Array|MakeArray "What do you mean?")))
                                                          (switch Utilities|FlowControl|Switch|SwitchonEnum_DialogueState _state_8
                                                            (:NewEnumerator0
                                                              (switch int _optionindex_8
                                                                (:0
                                                                  (bind (_state_9 _optionindex_9) (CallFunction|AddDialogue "Little Joe" "I know the dude you are talking about. I know it due to some really fucked up connections." (Utilities|Array|MakeArray "Continue. ")))
                                                                  (switch Utilities|FlowControl|Switch|SwitchonEnum_DialogueState _state_9
                                                                    (:NewEnumerator0
                                                                      (switch int _optionindex_9
                                                                        (:0
                                                                          (bind (_state_10 _optionindex_10) (CallFunction|AddDialogue "Little Joe" "They asked me to kill him but i refused." (Utilities|Array|MakeArray "Continue")))
                                                                          (switch Utilities|FlowControl|Switch|SwitchonEnum_DialogueState _state_10
                                                                            (:NewEnumerator0
                                                                              (switch int _optionindex_10
                                                                                (:0
                                                                                  (bind (_state_11 _optionindex_11) (CallFunction|AddDialogue "Little Joe" "I ain’t doing anything for them ever again. You should leave." (Utilities|Array|MakeArray "No wait, they plan on killing you." "Please all i need is a small lead.")))
                                                                                  (switch Utilities|FlowControl|Switch|SwitchonEnum_DialogueState _state_11
                                                                                    (:NewEnumerator0
                                                                                      (switch int _optionindex_11
                                                                                        (:0
                                                                                          (bind (_state_12 _optionindex_12) (CallFunction|AddDialogue "Little Joe" "A lot of people do, I’ll be fine." (Utilities|Array|MakeArray "No they WILL kill you.")))
                                                                                          (switch Utilities|FlowControl|Switch|SwitchonEnum_DialogueState _state_12
                                                                                            (:NewEnumerator0
                                                                                              (switch int _optionindex_12
                                                                                                (:0
                                                                                                  (bind (_state_13 _optionindex_13) (CallFunction|AddDialogue "Little Joe" "Who?" (Utilities|Array|MakeArray "I don’t know yet, someone. It might be the “lunatics” that you were talking about.")))
                                                                                                  (switch Utilities|FlowControl|Switch|SwitchonEnum_DialogueState _state_13
                                                                                                    (:NewEnumerator0
                                                                                                      (switch int _optionindex_13
                                                                                                        (:0
                                                                                                          (bind (_state_14 _optionindex_14) (CallFunction|AddDialogue "Little Joe" "No, they gain nothing from it. If someone is out to get me its the Iron Hounds." (Utilities|Array|MakeArray "Continue")))
                                                                                                          (switch Utilities|FlowControl|Switch|SwitchonEnum_DialogueState _state_14
                                                                                                            (:NewEnumerator0
                                                                                                              (switch int _optionindex_14
                                                                                                                (:0
                                                                                                                  (bind (_state_15 _optionindex_15) (CallFunction|AddDialogue "Little Joe" "But I will make sure that I am the last thing that each and every one of those fuckers see." (Utilities|Array|MakeArray "Continue")))
                                                                                                                  (switch Utilities|FlowControl|Switch|SwitchonEnum_DialogueState _state_15
                                                                                                                    (:NewEnumerator0
                                                                                                                      (switch int _optionindex_15
                                                                                                                        (:0
                                                                                                                          (bind (_state_16 _optionindex_16) (CallFunction|AddDialogue "Little Joe" "Now get out before I lose my temper." (Utilities|Array|MakeArray "Leave")))
                                                                                                                          (switch Utilities|FlowControl|Switch|SwitchonEnum_DialogueState _state_16
                                                                                                                            (:NewEnumerator0
                                                                                                                              (switch int _optionindex_16
                                                                                                                                (:0
                                                                                                                                  (Variables|/Game/TopDown/Blueprints/BP_TopDownGameMode.BP_TopDownGameMode_C|SetPlayerKicked (Variables|Default|GetGamemode) true)
                                                                                                                                  (Variables|/Game/TopDown/Blueprints/BP_TopDownGameMode.BP_TopDownGameMode_C|SetTimeSlot (Variables|Default|GetGamemode) 0)
                                                                                                                                  (CallFunction|CloseConversation))))))))))))))))))))))
                                                                                        (:1
                                                                                          (bind (_state_17 _optionindex_17) (CallFunction|AddDialogue "Little Joe" "You’d be better off letting it go." (Utilities|Array|MakeArray "Continue")))
                                                                                          (switch Utilities|FlowControl|Switch|SwitchonEnum_DialogueState _state_17
                                                                                            (:NewEnumerator0
                                                                                              (switch int _optionindex_17
                                                                                                (:0
                                                                                                  (bind (_state_18 _optionindex_18) (CallFunction|AddDialogue "Little Joe" "Trust me if you knew what you were going into, you would thank me." (Utilities|Array|MakeArray "Continue")))
                                                                                                  (switch Utilities|FlowControl|Switch|SwitchonEnum_DialogueState _state_18
                                                                                                    (:NewEnumerator0
                                                                                                      (switch int _optionindex_18
                                                                                                        (:0
                                                                                                          (bind (_state_19 _optionindex_19) (CallFunction|AddDialogue "Little Joe" "Now leave..." (Utilities|Array|MakeArray "Leave")))
                                                                                                          (switch Utilities|FlowControl|Switch|SwitchonEnum_DialogueState _state_19
                                                                                                            (:NewEnumerator0
                                                                                                              (switch int _optionindex_19
                                                                                                                (:0
                                                                                                                  (Variables|/Game/TopDown/Blueprints/BP_TopDownGameMode.BP_TopDownGameMode_C|SetPlayerKicked (Variables|Default|GetGamemode) true)
                                                                                                                  (CallFunction|CloseConversation))))))))))))))))))))))))))))))))))))))))))))))))))))))))))