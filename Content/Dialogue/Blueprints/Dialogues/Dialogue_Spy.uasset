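; Dialogue Blueprint for the Shady Man, an informant NPC whom the player can ask about gang leader Little Joe.
; BeginPlay fetches the game mode, and Dialogue branches on its TimeSlot (only slot 0 is scripted) and Key2 flag.
; Chained AddDialogue nodes form the keyless tree, which loops on small talk and sets NoKey2ConvoHappened after the Joe inquiry to give a brush-off later.
; The Key2 menu adds a favors option, but its choices are unwired.
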(event EventBeginPlay
  (CallFunction|GetGamemode))

(event EventTick
  (params (DeltaSeconds :type Float%20%28single-precision%29)))

(fn Dialogue
  (|CallParentFunction)
  (switch int (Variables|/Game/TopDown/Blueprints/BP_TopDownGameMode.BP_TopDownGameMode_C|GetTimeSlot (Variables|Default|GetGamemode))
    (:0
      (if (Variables|/Game/TopDown/Blueprints/BP_TopDownGameMode.BP_TopDownGameMode_C|GetKey2 (Variables|Default|GetGamemode))
        (bind (_state _optionindex) (CallFunction|AddDialogue "Shady Man" "Anything I can assist you with?" (Utilities|Array|MakeArray "Looking for a man that goes by the name Little Joe." "You look really shady. If you are really doing something illegal you should change your approach." "Zeal Devin sent me. I need 3 favors." "No.(Leave)")))
        (switch Utilities|FlowControl|Switch|SwitchonEnum_DialogueState _state
          (:NewEnumerator0
            (switch int _optionindex)))
        (elif (Variables|Default|GetNoKey2ConvoHappened)
          (bind (_state_2 _optionindex_2) (CallFunction|AddDialogue "Shady Man" "Can't get any information right now." (Utilities|Array|MakeArray "Continue")))
          (switch Utilities|FlowControl|Switch|SwitchonEnum_DialogueState _state_2
            (:NewEnumerator0
              (switch int _optionindex_2
                (:0
                  (CallFunction|ClearDialogueProgress)
                  (CallFunction|CloseConversation)))))
          (else
            (bind (_state_3 _optionindex_3) (CallFunction|AddDialogue "Shady Man" "Anything I can assist you with?" (Utilities|Array|MakeArray "Looking for a man that goes by the name Little Joe." "You look really shady. If you are really doing something illegal you should change your approach." "No.(Leave)") :!label _label))
            (switch Utilities|FlowControl|Switch|SwitchonEnum_DialogueState _state_3
              (:NewEnumerator0
                (switch int _optionindex_3
                  (:0
                    (bind (_state_4 _optionindex_4) (CallFunction|AddDialogue "Shady Man" "And you are?" (Utilities|Array|MakeArray "Lyen")))
                    (switch Utilities|FlowControl|Switch|SwitchonEnum_DialogueState _state_4
                      (:NewEnumerator0
                        (switch int _optionindex_4
                          (:0
                            (bind (_state_5 _optionindex_5) (CallFunction|AddDialogue "Shady Man" "So Lyen. Why would I give any information about a gang leader to a random detective." (Utilities|Array|MakeArray "Wait, how do you know?")))
                            (switch Utilities|FlowControl|Switch|SwitchonEnum_DialogueState _state_5
                              (:NewEnumerator0
                                (switch int _optionindex_5
                                  (:0
                                    (bind (_state_6 _optionindex_6) (CallFunction|AddDialogue "Shady Man" "I can see it in the way you walk. You rushed inside, looked all round the bar starting from a corner and touched every single thing." (Utilities|Array|MakeArray "Now don’t mind me but I better keep to myself. I am sure everyone loves me more with my tounge intact. ")))
                                    (switch Utilities|FlowControl|Switch|SwitchonEnum_DialogueState _state_6
                                      (:NewEnumerator0
                                        (switch int _optionindex_6
                                          (:0
                                            (Variables|Default|SetNoKey2ConvoHappened true)
                                            (CallFunction|ClearDialogueProgress)
                                            (CallFunction|CloseConversation))))))))))))))
                  (:1
                    (bind (_state_7 _optionindex_7) (CallFunction|AddDialogue "Shady Man" "Ah but you see i need to look shady." (Utilities|Array|MakeArray "Continue")))
                    (switch Utilities|FlowControl|Switch|SwitchonEnum_DialogueState _state_7
                      (:NewEnumerator0
                        (switch int _optionindex_7
                          (:0
                            (bind (_state_8 _optionindex_8) (CallFunction|AddDialogue "Shady Man" "Otherwise folk like you might get a little bored." (Utilities|Array|MakeArray "Continue")))
                            (switch Utilities|FlowControl|Switch|SwitchonEnum_DialogueState _state_8
                              (:NewEnumerator0
                                (switch int _optionindex_8
                                  (:0
                                    (bind (_state_9 _optionindex_9) (CallFunction|AddDialogue "Shady Man" "Look even if I was doing anything wrong, you would never know. So drop it." (Utilities|Array|MakeArray "Continue")))
                                    (switch Utilities|FlowControl|Switch|SwitchonEnum_DialogueState _state_9
                                      (:NewEnumerator0
                                        (switch int _optionindex_9
                                          (:0
                                            (goto _label))))))))))))))
                  (:2
                    (CallFunction|ClearDialogueProgress)
                    (CallFunction|CloseConversation)))))))))))

(fn GetGamemode
  (|CallParentFunction))