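; Bartender NPC dialogue for Aemon, where Lyen asks about Little Joe and can uncover Aemon's Beirien identity.
; The Dialogue override branches on gamemode time slot, alignment and key flags, plus whether they have met.
; Chained AddDialogue calls continue on Pass Through by option index; endings clear progress, some setting KeyA, DialogueHappened or advancing time.
; The good-alignment return menu's option handling is disconnected, so its choices lead nowhere.
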(event EventBeginPlay
  (CallFunction|GetGamemode))

(event EventTick
  (params (DeltaSeconds :type Float%20%28single-precision%29)))

(fn Dialogue
  (|CallParentFunction)
  (switch int (Variables|/Game/TopDown/Blueprints/BP_TopDownGameMode.BP_TopDownGameMode_C|GetTimeSlot (Variables|Default|GetGamemode))
    (:0
      (if (Variables|Default|GetDialogueHappened)
        (if (not (Variables|/Game/TopDown/Blueprints/BP_TopDownGameMode.BP_TopDownGameMode_C|GetKeyA (Variables|Default|GetGamemode)))
          (switch int (Variables|/Game/TopDown/Blueprints/BP_TopDownGameMode.BP_TopDownGameMode_C|GetGood/Bad/Ugly (Variables|Default|GetGamemode))
            (:0
              (bind (_state _optionindex) (CallFunction|AddDialogue "Aemon the Bartender " "What can I get you?" (Utilities|Array|MakeArray "Hey there Aemon, how are stuff?" "I will take a Ward Eight. (GOOD)" "My friend is missing and I need your help to get him back." "Nevermind.(Leave)") :!label _label)))
            (:1
              (bind (_state_2 _optionindex_2) (CallFunction|AddDialogue "Aemon the Bartender " "What can I get you?" (Utilities|Array|MakeArray "Hey there Aemon, how are stuff?" "My friend is missing and I need your help to get him back." "Nevermind.(Leave)") :!label _label_2))
              (switch Utilities|FlowControl|Switch|SwitchonEnum_DialogueState _state_2
                (:NewEnumerator0
                  (switch int _optionindex_2
                    (:0
                      (bind (_state_3 _optionindex_3) (CallFunction|AddDialogue "Aemon the Bartender" "Do I know you?" (Utilities|Array|MakeArray "Not yet.")))
                      (switch Utilities|FlowControl|Switch|SwitchonEnum_DialogueState _state_3
                        (:NewEnumerator0
                          (switch int _optionindex_3
                            (:0
                              (bind (_state_4 _optionindex_4) (CallFunction|AddDialogue "Aemon the Bartender" "And you know my name because?" (Utilities|Array|MakeArray "I just heard people calling you that.")))
                              (switch Utilities|FlowControl|Switch|SwitchonEnum_DialogueState _state_4
                                (:NewEnumerator0
                                  (switch int _optionindex_4
                                    (:0
                                      (switch int (Variables|/Game/TopDown/Blueprints/BP_TopDownGameMode.BP_TopDownGameMode_C|GetGood/Bad/Ugly (Variables|Default|GetGamemode))
                                        (:0
                                          (bind (_state_5 _optionindex_5) (CallFunction|AddDialogue "Aemon the Bartender" "Aight whatever. You want something to drink or are you just here to creep me off." (Utilities|Array|MakeArray "I actually need your help with something Aemon." "I will take a Ward Eight. (GOOD)")))
                                          (switch Utilities|FlowControl|Switch|SwitchonEnum_DialogueState _state_5
                                            (:NewEnumerator0
                                              (switch int _optionindex_5
                                                (:0
                                                  (bind (_state_6 _optionindex_6) (CallFunction|AddDialogue "Aemon the Bartender" "Best I can do is serve some drinks." (Utilities|Array|MakeArray "Continue") :!label _label_3))
                                                  (switch Utilities|FlowControl|Switch|SwitchonEnum_DialogueState _state_6
                                                    (:NewEnumerator0
                                                      (switch int _optionindex_6
                                                        (:0
                                                          (bind (_state_7 _optionindex_7) (CallFunction|AddDialogue "Aemon the Bartender" "So if that is not what you are looking for when you say “help”, I don’t know how useful I can be." (Utilities|Array|MakeArray "My friend is missing and I know you can help. Just put in a good word or two with Little Joe for me. Tell him I have an urgent business.")))
                                                          (switch Utilities|FlowControl|Switch|SwitchonEnum_DialogueState _state_7
                                                            (:NewEnumerator0
                                                              (switch int _optionindex_7
                                                                (:0
                                                                  (bind (_state_8 _optionindex_8) (CallFunction|AddDialogue "Aemon the Bartender" "Look I don’t know why you even think Joe and I are on good terms but even I could help, I made a promise not to get into this sort of business anymore." (Utilities|Array|MakeArray "Continue")))
                                                                  (switch Utilities|FlowControl|Switch|SwitchonEnum_DialogueState _state_8
                                                                    (:NewEnumerator0
                                                                      (switch int _optionindex_8
                                                                        (:0
                                                                          (bind (_state_9 _optionindex_9) (CallFunction|AddDialogue "Aemon the Bartender" "Hope you can understand. I am just looking out for myself." (Utilities|Array|MakeArray "Continue")))
                                                                          (switch Utilities|FlowControl|Switch|SwitchonEnum_DialogueState _state_9
                                                                            (:NewEnumerator0
                                                                              (switch int _optionindex_9
                                                                                (:0
                                                                                  (switch int (Variables|/Game/TopDown/Blueprints/BP_TopDownGameMode.BP_TopDownGameMode_C|GetGood/Bad/Ugly (Variables|Default|GetGamemode))
                                                                                    (:0
                                                                                      (goto _label))
                                                                                    (:1
                                                                                      _)
                                                                                    (:2
                                                                                      (Variables|/Game/TopDown/Blueprints/BP_TopDownGameMode.BP_TopDownGameMode_C|SetTimeSlot (Variables|Default|GetGamemode) 1)))
                                                                                  (CallFunction|ClearDialogueProgress)
                                                                                  (CallFunction|CloseConversation))))))))))))))))))
                                                (:1
                                                  (bind (_state_10 _optionindex_10) (CallFunction|AddDialogue "Aemon the Bartender" "Good choice. Coming right up." (Utilities|Array|MakeArray "Continue")))
                                                  (switch Utilities|FlowControl|Switch|SwitchonEnum_DialogueState _state_10
                                                    (:NewEnumerator0
                                                      (switch int _optionindex_10
                                                        (:0
                                                          (if (Variables|/Game/TopDown/Blueprints/BP_TopDownGameMode.BP_TopDownGameMode_C|GetKey2 (Variables|Default|GetGamemode))
                                                            (bind (_state_11 _optionindex_11) (CallFunction|AddDialogue "Lyen Thinks:" "Maybe I can ask him something personal, It might be useful later." (Utilities|Array|MakeArray "Continue")))
                                                            (switch Utilities|FlowControl|Switch|SwitchonEnum_DialogueState _state_11
                                                              (:NewEnumerator0
                                                                (switch int _optionindex_11
                                                                  (:0
                                                                    _))))
                                                            (else
                                                              (bind (_state_12 _optionindex_12) (CallFunction|AddDialogue "Lyen Thinks:" "Maybe I can ask him about this Joe person.)" (Utilities|Array|MakeArray "Continue")))
                                                              (switch Utilities|FlowControl|Switch|SwitchonEnum_DialogueState _state_12
                                                                (:NewEnumerator0
                                                                  (switch int _optionindex_12
                                                                    (:0
                                                                      _))))))
                                                          (bind (_state_13 _optionindex_13) (CallFunction|AddDialogue "Aemon the Bartender" "Here you go. Enjoy." (Utilities|Array|MakeArray "Wait how could I have missed it. Those eyes, that name, that slight accent... You are a Beirien aren’t you.")))
                                                          (switch Utilities|FlowControl|Switch|SwitchonEnum_DialogueState _state_13
                                                            (:NewEnumerator0
                                                              (switch int _optionindex_13
                                                                (:0
                                                                  (CallFunction|AddDialogue "Aemon the Bartender" "..." (Utilities|Array|MakeArray "How did you fool so many people, even I thought your kind didn’t exist anymore on these parts."))
                                                                  (bind (_state_14 _optionindex_14) (CallFunction|AddDialogue "You say “kind” as if we are any different from your “kind”." "Here you go. Enjoy." (Utilities|Array|MakeArray "Continue")))
                                                                  (switch Utilities|FlowControl|Switch|SwitchonEnum_DialogueState _state_14
                                                                    (:NewEnumerator0
                                                                      (switch int _optionindex_14
                                                                        (:0
                                                                          (bind (_state_15 _optionindex_15) (CallFunction|AddDialogue "Aemon the Bartender" "Despite all those things you said, it took you a while to figure out.." (Utilities|Array|MakeArray "Continue")))
                                                                          (switch Utilities|FlowControl|Switch|SwitchonEnum_DialogueState _state_15
                                                                            (:NewEnumerator0
                                                                              (switch int _optionindex_15
                                                                                (:0
                                                                                  (bind (_state_16 _optionindex_16) (CallFunction|AddDialogue "Aemon the Bartender" "No one that i served could even see through it. If all of these are not proof that we are not that different from your “kind”, then i don’t know what is." (Utilities|Array|MakeArray "Maybe I should call the police, I can see a phonebooth just that way." "Relax, I was against the way your people were treated, I wouldn’t try anything." "So how does hivemind work exactly. Does it just feel like someone else is controlling your brain.") :!label _label_4))
                                                                                  (switch Utilities|FlowControl|Switch|SwitchonEnum_DialogueState _state_16
                                                                                    (:NewEnumerator0
                                                                                      (switch int _optionindex_16
                                                                                        (:0
                                                                                          (bind (_state_17 _optionindex_17) (CallFunction|AddDialogue "Aemon the Bartender" "They are done with us. I still don’t know what they wanted from us, but they got it." (Utilities|Array|MakeArray "I’d imagine it has something to do with the wierd brain magic.")))
                                                                                          (switch Utilities|FlowControl|Switch|SwitchonEnum_DialogueState _state_17
                                                                                            (:NewEnumerator0
                                                                                              (switch int _optionindex_17
                                                                                                (:0
                                                                                                  (bind (_state_18 _optionindex_18) (CallFunction|AddDialogue "Aemon the Bartender" "If they really wanted to do experiments on us they would accept more refugees." (Utilities|Array|MakeArray "Continue")))
                                                                                                  (switch Utilities|FlowControl|Switch|SwitchonEnum_DialogueState _state_18
                                                                                                    (:NewEnumerator0
                                                                                                      (switch int _optionindex_18
                                                                                                        (:0
                                                                                                          (bind (_state_19 _optionindex_19) (CallFunction|AddDialogue "Aemon the Bartender" "There are thousands of unshackled Beiriens that suffer overseas. And they have accepted what, a hundred refugees in the span of a decade." (Utilities|Array|MakeArray "Continue")))
                                                                                                          (switch Utilities|FlowControl|Switch|SwitchonEnum_DialogueState _state_19
                                                                                                            (:NewEnumerator0
                                                                                                              (switch int _optionindex_19
                                                                                                                (:0
                                                                                                                  (goto _label_4))))))))))))))
                                                                                        (:1
                                                                                          (bind (_state_20 _optionindex_20) (CallFunction|AddDialogue "Aemon the Bartender" "Ah that is so good to know. I was kinda worried there for a second." (Utilities|Array|MakeArray "Continue")))
                                                                                          (switch Utilities|FlowControl|Switch|SwitchonEnum_DialogueState _state_20
                                                                                            (:NewEnumerator0
                                                                                              (switch int _optionindex_20
                                                                                                (:0
                                                                                                  (bind (_state_21 _optionindex_21) (CallFunction|AddDialogue "Aemon the Bartender" "If I something were to happen to me I really don’t know what my wife would have done." (Utilities|Array|MakeArray "Didn’t take you for a married man.")))
                                                                                                  (switch Utilities|FlowControl|Switch|SwitchonEnum_DialogueState _state_21
                                                                                                    (:NewEnumerator0
                                                                                                      (switch int _optionindex_21
                                                                                                        (:0
                                                                                                          (bind (_state_22 _optionindex_22) (CallFunction|AddDialogue "Aemon the Bartender" "I am though. Thats why I want stay out of any trouble. I don’t want to make Elisha unhappy." (Utilities|Array|MakeArray "Well maybe you should start wearing some lenses or glasses.")))
                                                                                                          (switch Utilities|FlowControl|Switch|SwitchonEnum_DialogueState _state_22
                                                                                                            (:NewEnumerator0
                                                                                                              (switch int _optionindex_22
                                                                                                                (:0
                                                                                                                  (Variables|/Game/TopDown/Blueprints/BP_TopDownGameMode.BP_TopDownGameMode_C|SetKeyA (Variables|Default|GetGamemode) true)
                                                                                                                  (bind (_state_23 _optionindex_23) (CallFunction|AddDialogue "Aemon the Bartender" "Thanks you are very kind." (Utilities|Array|MakeArray "Continue")))
                                                                                                                  (switch Utilities|FlowControl|Switch|SwitchonEnum_DialogueState _state_23
                                                                                                                    (:NewEnumerator0
                                                                                                                      (switch int _optionindex_23
                                                                                                                        (:0
                                                                                                                          (Variables|/Game/TopDown/Blueprints/BP_TopDownGameMode.BP_TopDownGameMode_C|SetTimeSlot (Variables|Default|GetGamemode) 1)
                                                                                                                          (CallFunction|ClearDialogueProgress)
                                                                                                                          (CallFunction|CloseConversation))))))))))))))))))
                                                                                        (:2
                                                                                          (bind (_state_24 _optionindex_24) (CallFunction|AddDialogue "Aemon the Bartender" "Don’t know, I was born unshackled. I am a mix and my father was also unshackled. I have no connection to the Order." (Utilities|Array|MakeArray "But yet you still inherited the bronze eye color.")))
                                                                                          (switch Utilities|FlowControl|Switch|SwitchonEnum_DialogueState _state_24
                                                                                            (:NewEnumerator0
                                                                                              (switch int _optionindex_24
                                                                                                (:0
                                                                                                  (bind (_state_25 _optionindex_25) (CallFunction|AddDialogue "Aemon the Bartender" "I don’t really get to choose, do I?" (Utilities|Array|MakeArray "Yeah but you could at least change your name.")))
                                                                                                  (switch Utilities|FlowControl|Switch|SwitchonEnum_DialogueState _state_25
                                                                                                    (:NewEnumerator0
                                                                                                      (switch int _optionindex_25
                                                                                                        (:0
                                                                                                          (bind (_state_26 _optionindex_26) (CallFunction|AddDialogue "Aemon the Bartender" "I am proud of the name I was given. Even if it gets me in a little trouble." (Utilities|Array|MakeArray "Continue")))
                                                                                                          (switch Utilities|FlowControl|Switch|SwitchonEnum_DialogueState _state_26
                                                                                                            (:NewEnumerator0
                                                                                                              (switch int _optionindex_26
                                                                                                                (:0
                                                                                                                  (goto _label_4))))))))))))))))))))))))))))))))))))))
                                        (:1
                                          (CallFunction|AddDialogue "Aemon the Bartender" "Aight whatever. You want something to drink or are you just here to creep me off." (Utilities|Array|MakeArray "I actually need your help with something Aemon.") :!label _label_5))
                                        (:2
                                          (goto _label_5))))))))))))
                    (:1
                      (goto _label_3))
                    (:2
                      (CallFunction|ClearDialogueProgress)
                      (CallFunction|CloseConversation))))))
            (:2
              (goto _label_2))))
        (else
          (bind (_state_27 _optionindex_27) (CallFunction|AddDialogue "Lyen" "Hey, I am looking for a man. Know anyone that goes by Little Joe?" (Utilities|Array|MakeArray "Continue")))
          (switch Utilities|FlowControl|Switch|SwitchonEnum_DialogueState _state_27
            (:NewEnumerator0
              (switch int _optionindex_27
                (:0
                  (bind (_state_28 _optionindex_28) (CallFunction|AddDialogue "Bartender" "Never heard of him." (Utilities|Array|MakeArray "Continue")))
                  (switch Utilities|FlowControl|Switch|SwitchonEnum_DialogueState _state_28
                    (:NewEnumerator0
                      (switch int _optionindex_28
                        (:0
                          (bind (_state_29 _optionindex_29) (CallFunction|AddDialogue "Bartender" "You want something to drink or are you only here to ask questions." (Utilities|Array|MakeArray "I’ll take whatever you recommend.")))
                          (switch Utilities|FlowControl|Switch|SwitchonEnum_DialogueState _state_29
                            (:NewEnumerator0
                              (switch int _optionindex_29
                                (:0
                                  (bind (_state_30 _optionindex_30) (CallFunction|AddDialogue "Bartender" "Coming right up." (Utilities|Array|MakeArray "Wait for the drink")))
                                  (switch Utilities|FlowControl|Switch|SwitchonEnum_DialogueState _state_30
                                    (:NewEnumerator0
                                      (switch int _optionindex_30
                                        (:0
                                          (bind (_state_31 _optionindex_31) (CallFunction|AddDialogue "Lyen" "Weird, I was sure the bartender would know something. He looked somewhat worried when i asked him about the bartender. Maybe I could try to push it..." (Utilities|Array|MakeArray "Continue")))
                                          (switch Utilities|FlowControl|Switch|SwitchonEnum_DialogueState _state_31
                                            (:NewEnumerator0
                                              (switch int _optionindex_31
                                                (:0
                                                  (bind (_state_32 _optionindex_32) (CallFunction|AddDialogue "Bartender" "Here is your Ward Eight, enjoy." (Utilities|Array|MakeArray "If you don’t mind me asking, what is your name." "You were very quick to dismiss my question, there could be something in it for you as well.") :!label _label_6))
                                                  (switch Utilities|FlowControl|Switch|SwitchonEnum_DialogueState _state_32
                                                    (:NewEnumerator0
                                                      (switch int _optionindex_32
                                                        (:0
                                                          (bind (_state_33 _optionindex_33) (CallFunction|AddDialogue "Aemon the Bartender" "My name is Aemon, and yours is?" (Utilities|Array|MakeArray "I am Lyen.")))
                                                          (switch Utilities|FlowControl|Switch|SwitchonEnum_DialogueState _state_33
                                                            (:NewEnumerator0
                                                              (switch int _optionindex_33
                                                                (:0
                                                                  (bind (_state_34 _optionindex_34) (CallFunction|AddDialogue "Aemon the Bartender" "Nice to meet you, Lyen." (Utilities|Array|MakeArray "Likewise. Your name is pretty exotic, where are you from?")))
                                                                  (switch Utilities|FlowControl|Switch|SwitchonEnum_DialogueState _state_34
                                                                    (:NewEnumerator0
                                                                      (switch int _optionindex_34
                                                                        (:0
                                                                          (bind (_state_35 _optionindex_35) (CallFunction|AddDialogue "Aemon the Bartender" "Some boring old town. My mom saw my name in a book and thought it was cool." (Utilities|Array|MakeArray "Your mom sounds like a cool lady")))
                                                                          (switch Utilities|FlowControl|Switch|SwitchonEnum_DialogueState _state_35
                                                                            (:NewEnumerator0
                                                                              (switch int _optionindex_35
                                                                                (:0
                                                                                  (bind (_state_36 _optionindex_36) (CallFunction|AddDialogue "Aemon the Bartender" "That she is." (Utilities|Array|MakeArray "Continue")))
                                                                                  (switch Utilities|FlowControl|Switch|SwitchonEnum_DialogueState _state_36
                                                                                    (:NewEnumerator0
                                                                                      (switch int _optionindex_36
                                                                                        (:0
                                                                                          (bind (_state_37 _optionindex_37) (CallFunction|AddDialogue "Aemon the Bartender" "Listen, you look like a half decent fellow so let me give you some advice." (Utilities|Array|MakeArray "Continue")))
                                                                                          (switch Utilities|FlowControl|Switch|SwitchonEnum_DialogueState _state_37
                                                                                            (:NewEnumerator0
                                                                                              (switch int _optionindex_37
                                                                                                (:0
                                                                                                  (bind (_state_38 _optionindex_38) (CallFunction|AddDialogue "Aemon the Bartender" "Whoever you think this Little Joe dude is, that ain’t him. He is simply trouble." (Utilities|Array|MakeArray "Continue")))
                                                                                                  (switch Utilities|FlowControl|Switch|SwitchonEnum_DialogueState _state_38
                                                                                                    (:NewEnumerator0
                                                                                                      (switch int _optionindex_38
                                                                                                        (:0
                                                                                                          (bind (_state_39 _optionindex_39) (CallFunction|AddDialogue "Aemon the Bartender" "It’s not worth chasing trouble like that for a few pennies. So I will serve you some drinks, and when you are done with them you will leave." (Utilities|Array|MakeArray "It’s not what you think. You should at least give me a chance, it is not the pennies that I am after.")))
                                                                                                          (switch Utilities|FlowControl|Switch|SwitchonEnum_DialogueState _state_39
                                                                                                            (:NewEnumerator0
                                                                                                              (switch int _optionindex_39
                                                                                                                (:0
                                                                                                                  (bind (_state_40 _optionindex_40) (CallFunction|AddDialogue "Aemon the Bartender" "Still i can’t help you, made a promise to keep myself out of trouble." (Utilities|Array|MakeArray "Continue")))
                                                                                                                  (switch Utilities|FlowControl|Switch|SwitchonEnum_DialogueState _state_40
                                                                                                                    (:NewEnumerator0
                                                                                                                      (switch int _optionindex_40
                                                                                                                        (:0
                                                                                                                          (bind (_state_41 _optionindex_41) (CallFunction|AddDialogue "Aemon the Bartender" "But you should try and talk to other people. Maybe go play some pool, that could help you think." (Utilities|Array|MakeArray "Thanks Aemon. ")))
                                                                                                                          (switch Utilities|FlowControl|Switch|SwitchonEnum_DialogueState _state_41
                                                                                                                            (:NewEnumerator0
                                                                                                                              (switch int _optionindex_41
                                                                                                                                (:0
                                                                                                                                  (Variables|Default|SetDialogueHappened true)
                                                                                                                                  (Variables|/Game/TopDown/Blueprints/BP_TopDownGameMode.BP_TopDownGameMode_C|SetTimeSlot (Variables|Default|GetGamemode) 1)
                                                                                                                                  (CallFunction|ClearDialogueProgress)
                                                                                                                                  (CallFunction|CloseConversation))))))))))))))))))))))))))))))))))))))
                                                        (:1
                                                          (bind (_state_42 _optionindex_42) (CallFunction|AddDialogue "Bartender" "Nope. There ain’t." (Utilities|Array|MakeArray "Continue")))
                                                          (switch Utilities|FlowControl|Switch|SwitchonEnum_DialogueState _state_42
                                                            (:NewEnumerator0
                                                              (switch int _optionindex_42
                                                                (:0
                                                                  (bind (_state_43 _optionindex_43) (CallFunction|AddDialogue "Bartender" "Also like I said. I am just a guy who pours drinks, I know nothing." (Utilities|Array|MakeArray "Continue")))
                                                                  (switch Utilities|FlowControl|Switch|SwitchonEnum_DialogueState _state_43
                                                                    (:NewEnumerator0
                                                                      (switch int _optionindex_43
                                                                        (:0
                                                                          (goto _label_6))))))))))))))))))))))))))))))))))))
    (:1
      (bind (_state_44 _optionindex_44) (CallFunction|AddDialogue "Lyen" "It is way too crowded, no way you can get to talk to him." (Utilities|Array|MakeArray "Continue")))
      (switch Utilities|FlowControl|Switch|SwitchonEnum_DialogueState _state_44
        (:NewEnumerator0
          (switch int _optionindex_44
            (:0
              (Variables|/Game/TopDown/Blueprints/BP_TopDownGameMode.BP_TopDownGameMode_C|SetTimeSlot (Variables|Default|GetGamemode) 1)
              (CallFunction|ClearDialogueProgress)
              (CallFunction|CloseConversation))))))
    (:2
      (bind (_state_45 _optionindex_45) (CallFunction|AddDialogue "Lyen" "He is in the back cleaning dishes. He aint coming back anytime soon." (Utilities|Array|MakeArray "Continue")))
      (switch Utilities|FlowControl|Switch|SwitchonEnum_DialogueState _state_45
        (:NewEnumerator0
          (switch int _optionindex_45
            (:0
              (CallFunction|ClearDialogueProgress)
              (CallFunction|CloseConversation))))))))

(fn GetGamemode
  (|CallParentFunction))